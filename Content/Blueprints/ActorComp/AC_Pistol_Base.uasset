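; AC_Pistol_Base is a base pistol weapon that fires physics-driven bullets when UseWeapon is triggered.
; UseWeapon passes the shooter's rotation to Shoot, which spawns a scaled-up BP_Bullet at the gun mesh's muzzle socket and launches it with a forward impulse.
; An empty Mag calls Reload, which only prints a placeholder error, and Shoot never decrements Mag.
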(event `/Game/Blueprints/Interfaces/I_Weapon.UseWeapon`
  (params (ShooterTransform :type "Transform Structure"))
  (`KismetSystemLibrary.PrintString` "Gun: Pew")
  (`self.Shoot` (.rotation ShooterTransform)))

(fn `Reload`
  (`KismetSystemLibrary.PrintString` "Error: Logic not added yet"))

(fn `Shoot`
  (params (AimRotation :type "Rotator Structure"))
  (locals (AimInput :type "Rotator Structure"))
  (if (> (`self.Mag`) 0)
    (set `local.AimInput` AimRotation)
    (bind _returnvalue (`|SpawnActorFromClass` "/Game/Blueprints/BP_Bullet.BP_Bullet_C" (`KismetMathLibrary.MakeTransform` (`SkeletalMeshSocket.GetSocketLocation` (`SkinnedAsset.FindSocket` (`self.GunMesh`) "Socket_Muzzle") null) (`local.AimInput`) (10.0 10.0 10.0)) "AlwaysSpawn" "MultiplyWithRoot" null null))
    (bind _staticmesh (`/Game/Blueprints/BP_Bullet.StaticMesh` _returnvalue))
    (`PrimitiveComponent.AddImpulse` _staticmesh (* (`SceneComponent.GetForwardVector` _staticmesh) 1000.0) "None" false)
    (else
      (`self.Reload`))))